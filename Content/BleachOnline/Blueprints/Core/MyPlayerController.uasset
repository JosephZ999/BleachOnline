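; Player controller for BleachOnline that drives character selection and UI setup.
; Custom events create the character selector, with mouse cursor and a selection callback, and the input widget.
; OnSelected passes the player and chosen hero to MyGameMode's OnPlayerReady, while Possess triggers BOHUD initialization through InitGameUI.
; The input-mode switches for both widgets are left disconnected and never run.
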(event `ShowSelectorWidget`
  (bind _returnvalue (`|CreateWidget` "/Game/BleachOnline/Blueprints/UI/CharacterSelector.CharacterSelector_C"))
  (`UserWidget.AddToViewport` _returnvalue 0)
  (set `PlayerController.bShowMouseCursor` true (`GameplayStatics.GetPlayerController` 0))
  (add `/Game/BleachOnline/Blueprints/UI/CharacterSelector.OnCharSelected` _returnvalue (`|CreateDelegate` :!event `OnSelected`)))

(event `ShowInputWidget`
  (bind _returnvalue (`|CreateWidget` "/Game/BleachOnline/Blueprints/UI/Input.Input_C"))
  (`UserWidget.AddToViewport` _returnvalue 0))

(event `OnSelected`
  (params (Player :type "PlayerController Object Reference") (NewParam :type Integer))
  (bind _asmy_game_mode (cast `/Game/BleachOnline/Blueprints/Core/MyGameMode` (`GameplayStatics.GetGameMode`)))
  (`/Game/BleachOnline/Blueprints/Core/MyGameMode.OnPlayerReady` _asmy_game_mode Player NewParam))

(event `self.ReceivePossess`
  (params (PossessedPawn :type "Pawn Object Reference"))
  (`self.InitGameUI`))

(event `InitGameUI`
  (bind _asbohud (cast `BOHUD` (`self.GetHUD`)))
  (`BOHUD.Initialize` _asbohud))

(fn `UserConstructionScript`)