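; Base character Blueprint for BleachOnline that handles movement, two-way facing, jumping and a test-style launch.
; Tick feeds forward and right axes into world-space movement, snapping control yaw to the sign of X and counter-rotating ArmComp to offset the flip.
; It also draws debug lines for move vector and velocity direction.
; Space jumps, while Z launches the character along fixed world +X, regardless of facing.
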(event `self.ReceiveTick`
  (params (DeltaSeconds :type "Float (single-precision)"))
  (bind _returnvalue (`self.GetController`))
  (bind _returnvalue_2 (`KismetMathLibrary.MakeRotator` 0.0))
  (bind _returnvalue_3 (`KismetMathLibrary.MakeRotator` 0.0 0.0 180.0))
  (bind _returnvalue_4 (`self.K2_GetActorLocation`))
  (bind _armcomp (`self.ArmComp`))
  (bind _returnvalue_5 (`KismetMathLibrary.MakeVector` (`self.GetInputAxisValue`) (`self.GetInputAxisValue`)))
  (`self.AddMovementInput` _returnvalue_5)
  (`|ExecutionSequence`
    (:`then_0`
      (`/Engine/EditorBlueprintResources/StandardMacros.CompareFloat` (`KismetMathLibrary.SignOfFloat` (.x _returnvalue_5))
        (:`>`
          (`Controller.SetControlRotation` _returnvalue _returnvalue_2)
          (`SceneComponent.K2_SetRelativeRotation` _armcomp _returnvalue_3 false false))
        (:`<`
          (`Controller.SetControlRotation` _returnvalue _returnvalue_3)
          (`SceneComponent.K2_SetRelativeRotation` _armcomp _returnvalue_2 false false))))
    (:`then_1`
      (`KismetSystemLibrary.DrawDebugLine` _returnvalue_4 (+ _returnvalue_4 (* (`BOCharacterMovementComponent.GetMoveVector` (`self.MovementComp`)) 100.0)) (struct :`G` 0.993179 :`B` 1.0 :`A` 1.0) 0.0 2.0)
      (`KismetSystemLibrary.DrawDebugLine` _returnvalue_4 (+ _returnvalue_4 (* (`KismetMathLibrary.Normal` (`self.GetVelocity`)) 100.0)) (struct :`R` 1.0 :`G` 0.411592 :`A` 1.0) 0.0 2.0))))

(event `Key|SpaceBar`
  (params (Key :type "Key Structure"))
  (:`Pressed`
    (`self.Jump`)))

(event `Key|Z`
  (params (Key :type "Key Structure"))
  (:`Pressed`
    (`self.LaunchCharacter` (`KismetMathLibrary.MakeVector` 1000.0))))

(fn `UserConstructionScript`)