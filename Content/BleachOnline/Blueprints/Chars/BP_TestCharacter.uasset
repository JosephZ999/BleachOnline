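; BP_TestCharacter is a test character Blueprint that drives the BOCharacterMovement component from player input.
; Each tick it builds a horizontal vector from the forward and right move values, passes it to the component as the movement vector, and prints the resulting velocity for debugging.
; Pressing the Jump action calls the component's jump.
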(event `self.ReceiveTick`
  (params (DeltaSeconds :type "Float (single-precision)"))
  (set `self.NewVar_0` (`KismetMathLibrary.MakeVector` (`self.GetInputAxisValue`) (`self.GetInputAxisValue`)))
  (`BOCharacterMovementComponent.SetMovementVector` (`self.BOCharacterMovement`) (`self.NewVar_0`) 1.0)
  (`KismetSystemLibrary.PrintString` (`KismetStringLibrary.Conv_VectorToString` (`BOCharacterMovementComponent.GetVelocity` (`self.BOCharacterMovement`)))))

(event `InputAction|Jump`
  (params (Key :type "Key Structure"))
  (:`Pressed`
    (`BOCharacterMovementComponent.Jump` (`self.BOCharacterMovement`))))

(fn `UserConstructionScript`)